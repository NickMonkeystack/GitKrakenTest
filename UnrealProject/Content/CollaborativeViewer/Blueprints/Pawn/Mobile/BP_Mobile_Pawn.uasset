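; Mobile pawn for the Collaborative Viewer that turns touch gestures into swipe and dolly input values.
; Update events compute per-update deltas for the first touch and the midpoint of two touches, flipping Y and storing previous positions.
; While both touches are pressed, the pinch axis yields a dolly delta, which otherwise resets to zero.
; The construction script attaches the TextName component to the camera.
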(event Custom|UpdateTouch1and2_Input_delta
  (bind _returnvalue (Game|GetPlayerController 0))
  (bind _touch1loc (Variables|Default|GetTouch1Loc))
  (bind (_x _y) (Math|Vector2D|BreakVector2D _touch1loc))
  (bind (_locationx _locationy) (Class|PlayerController|GetInputTouchState _returnvalue "Touch2"))
  (bind _returnvalue_2 (Math|Float|Lerp _y _locationy 0.5))
  (bind _returnvalue_3 (Math|Float|Lerp _x _locationx 0.5))
  (bind _returnvalue_4 (Math|Vector2D|MakeVector2D _returnvalue_3 _returnvalue_2))
  ;[0.2555 0.7775 1] Make Swipe Speed  touch1 and 2 Delta
  (Variables|Default|SetTwoTouchSwipeInput (* (- _returnvalue_4 (Variables|Default|GetPrevTouch1And2_Loc)) "(X=1.000000,Y=-1.000000)"))
  (Variables|Default|SetPrevTouch1And2_Loc _returnvalue_4))

(event Custom|UpdateTouch1_Input_Delta
  (bind _returnvalue (Game|GetPlayerController 0))
  (bind (_locationx _locationy) (Class|PlayerController|GetInputTouchState _returnvalue "Touch1"))
  (bind _returnvalue_2 (Math|Vector2D|MakeVector2D _locationx _locationy))
  ;[0.2555 0.7775 1] Make Swipe Delta touch1
  (Utilities|FlowControl|Sequence
    (:then_0
      (Utilities|FlowControl|DoOnce false
        (:Completed
          (Variables|Default|SetPrevTouch1Loc _returnvalue_2))))
    (:then_1
      _))
  (Variables|Default|SetTouch1Loc _returnvalue_2)
  (Variables|Default|SetSwipeInputDelta (* (- _returnvalue_2 (Variables|Default|GetPrevTouch1Loc)) "(X=1.000000,Y=-1.000000)"))
  (Variables|Default|SetPrevTouch1Loc _returnvalue_2))

(event Input|AxisEvents|InputAxispinch
  (params (AxisValue :type Float%20%28single-precision%29))
  (bind _returnvalue (- AxisValue 1.0))
  ;[0.2555 0.7775 1] ZOOM
  (if (and (Variables|Default|GetIsTouch1Pressed) (Variables|Default|GetIsTouch2Pressed))
    (Variables|Default|SetIsDolly true)
    (Variables|Default|SetDollyInput (- _returnvalue (Variables|Default|GetPreviousPinchValue)))
    (Variables|Default|SetPreviousPinchValue _returnvalue)
    (else
      (Variables|Default|SetIsDolly false)
      (Variables|Default|SetDollyInput 0.0)
      (Variables|Default|SetPreviousPinchValue 0.0))))

(fn ConstructionScript
  (Transformation|AttachComponentToComponent (Variables|Default|GetTextName) (Variables|Default|GetCamera) "None" "KeepRelative" "KeepRelative" "KeepRelative" true))