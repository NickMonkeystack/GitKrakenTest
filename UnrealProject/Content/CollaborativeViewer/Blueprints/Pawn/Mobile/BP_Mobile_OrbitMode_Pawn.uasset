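; Mobile orbit-mode pawn for the Collaborative Viewer, handling touch camera control and object manipulation.
; One finger orbits or taps to set an interest point; holding still runs a highlight timeline, then drags the hit actor; two fingers pinch-dolly and pan.
; Touch events set state flags that Tick, enabled on touch, uses to update camera, actor movement, laser and player-name facing.
; Highlight and laser updates go through server calls.
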(event Custom|TranslateActor
  (bind _returnvalue (Game|GetPlayerController 0))
  (bind _returnvalue_2 (Game|GetPlayerController 0))
  (bind (_locationx _locationy) (Class|PlayerController|GetInputTouchState _returnvalue_2 "Touch1"))
  (bind _returnvalue_3 (Math|Vector2D|MakeVector2D _locationx _locationy))
  (bind (_worldposition _worlddirection) (Class|GameplayStatics|DeprojectScreentoWorld _returnvalue _returnvalue_3))
  ;[0.2555 0.7775 1] Translate Actor
  (if (|Bool)
    (Default|MoveActor (Variables|Default|GetTransform) _worldposition _worlddirection 0.0)))

(event Custom|UpdateControlRotation
  (bind _returnvalue (Pawn|GetController))
  ;[0.2555 0.7775 1] Initial Spawn Rotation depending on PlayerStart rotation
  (Utilities|IsValid _returnvalue
    (:Is%20Valid
      (Pawn|SetControlRotation _returnvalue (Math|Rotator|MakeRotator 0.0 0.0 (Variables|Default|GetInitialControlRotation_0))))))

(event Custom|EventLookAtName
  ;[0.2555 0.7775 1] Update PlayerName direction. The name should always look towards the user's camera. Uses a shared function in the 'FL_PawnCommonFuntions' function library
  (CallFunction|RotatePlayerNamestoCamera self (Variables|Default|GetCamera)))

(event EventBeginPlay
  (bind _returnvalue (Game|GetPlayerController 0))
  ;[0.0146 1 0] Begin play
  (Utilities|FlowControl|Sequence
    (:then_0
      (Actor|Tick|SetActorTickEnabled false)
      (Variables|Default|SetCameraRotationSpeed 0.1)
      (Variables|Default|SetCameraDollySpeed 25.0)
      (Variables|Default|SetCameraPanSpeed 0.02)
      (Rendering|Material|SetScalarParameterValue "/Game/CollaborativeViewer/PostProcess/SelectableParams.SelectableParams" "SelectIntensity" 0.0 :!class /Script/Engine.KismetMaterialLibrary)
      (Class|PlayerController|ActivateTouchInterface (Game|GetPlayerController 0)))
    (:then_1
      (bind _returnvalue_2 (UserInterface|CreateWidget "/Game/CollaborativeViewer/UMG/GameMenu/OrbitTarget.OrbitTarget_C" (Game|GetPlayerController 0)))
      (bind _output_get (Variables|Default|SetOrbitTargetWidget _returnvalue_2))
      (UserInterface|Viewport|AddtoPlayerScreen _output_get))
    (:then_2
      (Class|WidgetBlueprintLibrary|SetFocustoGameViewport)
      (Variables|/Script/Engine.PlayerController|SetbShowMouseCursor _returnvalue true)
      (Variables|/Script/Engine.PlayerController|SetbEnableClickEvents _returnvalue true)
      (Variables|/Script/Engine.PlayerController|SetbEnableMouseOverEvents _returnvalue true))
    (:then_3
      (Variables|Default|SetPlayerMeshesArray (Utilities|Array|MakeArray 0 (Variables|Default|GetSplineMesh)))
      (CallFunction|SetupNameColor))))

(event EventTick
  (params (DeltaSeconds :type Float%20%28single-precision%29))
  (bind _camera (Variables|Default|GetCamera))
  ;[1 0.1326 0.09279] Update every frame only  when Interacting
  (Utilities|FlowControl|Sequence
    (:then_0
      (Utilities|FlowControl|Sequence
        (:then_0
          (CallFunction|UpdateTouch1InputDelta)
          (if (Variables|Default|GetTouch1)
            (CallFunction|UpdateLaserStartEndRunonServer (+ (Transformation|GetWorldLocation (Variables|Default|GetCamera)) "0,-5.000000,-10.000000") (Variables|Default|GetIntersectionLocation))))
        (:then_1
          ;;[1 1 1] CameraControl
          (CallFunction|OrbitCamera (Variables|Default|GetSwipeInputDelta))
          (CallFunction|CameraDolly _camera)
          (CallFunction|PanCamera (Variables|Default|GetSwipeInputDelta) _camera))
        (:then_2
          (CallFunction|TranslateActor))
        (:then_3
          (CallFunction|EventLookatName))))
    (:then_1
      (CallFunction|DisableTick true))))

(event Input|ActionEvents|InputActionPushAndPull
  (params (Key :type Key%20Structure))
  ;[0.2555 0.7775 1] MakeActorCloser
  (:Pressed
    (Variables|Default|SetActorOffsetLocation (+ (Variables|Default|GetActorOffsetLocation) (Class|Actor|GetInputAxisKeyValue)))))

(event Input|AxisEvents|InputAxispinch
  (params (AxisValue :type Float%20%28single-precision%29))
  (bind _returnvalue (- AxisValue 1.0))
  ;[0.2555 0.7775 1] ZOOM
  (if (and (Variables|Default|GetIsTouch1Pressed) (Variables|Default|GetIsTouch2Pressed))
    (Variables|Default|SetIsDolly true)
    (Variables|Default|SetDollyInput (- _returnvalue (Variables|Default|GetPreviousPinchValue)))
    (Variables|Default|SetPreviousPinchValue _returnvalue)
    (else
      (Variables|Default|SetIsDolly false)
      (Variables|Default|SetDollyInput 0.0)
      (Variables|Default|SetPreviousPinchValue 0.0))))

(event Input|TouchEvents|Touch2
  (params (Key :type Key%20Structure))
  ;[1 0.8299 0.2633] Touch 2
  (:Pressed
    (Variables|Default|SetIsTouch2Pressed true)
    (Variables|Default|SetPrevTouch1And2_Loc (|GetTouch1andtwomiddle_2_2_2))
    (Variables|Default|SetIsOrbiting false)
    (if (not (Variables|Default|GetIsObjectTranslating))
      (Variables|Default|SetIsDolly true)
      (Variables|Default|SetIsPanning true)))
  (:Released
    (Variables|Default|SetIsTouch2Pressed false)
    (Variables|Default|SetIsDolly false)
    (Variables|Default|SetIsPanning false)))

(event Input|MouseEvents|RightMouseButton
  (params (Key :type Key%20Structure))
  ;[1 0.8299 0.2633] Rotate
)

(event Input|TouchEvents|Touch1
  (params (Key :type Key%20Structure))
  (bind _returnvalue (|GetTouch1Location_2))
  ;[1 0.8299 0.2633] Touch 1
  (:Pressed
    (Utilities|FlowControl|Sequence
      (:then_0
        (Actor|Tick|SetActorTickEnabled true)
        (Variables|Default|SetIsTouch1Pressed true)
        (bind _output_get (Variables|Default|SetStartInteractingLocation _returnvalue))
        (Variables|Default|SetPrevTouch1Loc _output_get)
        (if (Variables|Default|GetIsInterestPointAnimDone)
          (CallFunction|SetHitActor (CallFunction|GetHit))
          (Variables|Default|SetIsOrbiting true)))
      (:then_1
        ;;[1 1 1] HighLight Actor
        (CallFunction|SetCustomDepthRunonServer (Variables|Default|GetCurrentHitActor) true)
        (bind _selectingf (Timeline|ItWillSelect PlayFromStart)
          (:Update
            (if (Variables|Default|GetIsTouch2Pressed)
              (Audio|Components|Audio|Stop (Variables|Default|GetItWillSelect) :!label _label)
              (Rendering|Material|SetScalarParameterValue "/Game/CollaborativeViewer/PostProcess/SelectableParams.SelectableParams" "SelectIntensity" 0.0 :!class /Script/Engine.KismetMaterialLibrary)
              (elif (Math|Vector|Equal(Vector) _returnvalue (Variables|Default|GetStartInteractingLocation) 1.0)
                (Rendering|Material|SetScalarParameterValue "/Game/CollaborativeViewer/PostProcess/SelectableParams.SelectableParams" "SelectIntensity" _selectingf :!class /Script/Engine.KismetMaterialLibrary)
                (else
                  (goto _label)))))
          (:Finished
            (Variables|Default|SetIsSelectStart true)
            (if (Variables|Default|GetIsTouch1Pressed)
              (Variables|Default|SetIsOrbiting false)
              (Variables|Default|SetIsObjectTranslating true)))))))
  (:Released
    (Audio|Components|Audio|Stop (Variables|Default|GetItWillSelect))
    (Rendering|Material|SetScalarParameterValue "/Game/CollaborativeViewer/PostProcess/SelectableParams.SelectableParams" "SelectIntensity" 0.0 :!class /Script/Engine.KismetMaterialLibrary)
    (CallFunction|SetCustomDepthRunonServer (Variables|Default|GetCurrentHitActor) false)
    (Variables|Default|SetStopInteractingLocation (|GetTouch_End_Location_2))
    (if (and (Math|Vector|Equal(Vector) (Variables|Default|GetStartInteractingLocation) (Variables|Default|GetStopInteractingLocation) 0.01) (not (Variables|Default|GetIsSelectStart)))
      (CallFunction|SetCameraInterestPoint))
    (Variables|Default|SetIsObjectTranslating false)
    (Variables|Default|SetIsOrbiting false)
    (Variables|Default|SetIsTouch1Pressed false)
    (Variables|Default|SetIsSelectStart false)))

(fn ConstructionScript
  (Transformation|AttachComponentToComponent (Variables|Default|GetTextName) (Variables|Default|GetCamera) "None" "KeepRelative" "KeepRelative" "KeepRelative" true))

(fn CheckforMouseDrag
  (bind _returnvalue (Game|GetPlayerController 0))
  (bind _initmousepos (Variables|Default|GetInitMousePos))
  (bind _dragmargin (Variables|Default|GetDragMargin))
  (bind _dragmargin_2 (Variables|Default|GetDragMargin))
  (bind (_locationx _locationy) (Game|Player|GetMousePosition _returnvalue))
  (if (Math|Boolean|ORBoolean (>= _locationx (+ (.x _initmousepos) _dragmargin)) (<= _locationy (- (.y _initmousepos) _dragmargin)) (>= _locationy (+ (.y _initmousepos) _dragmargin_2)) (<= _locationx (- (.x _initmousepos) _dragmargin_2)))
    _
    (elif (Variables|Default|GetisDragging)
      _
      (else
        (return false))))
  (Variables|Default|SetisDragging true)
  (return true))

(fn GetHit
  (return (.HitResult (Class|PlayerController|GetHitResultUnderCursorforObjects (Game|GetPlayerController 0) (Utilities|Array|MakeArray "ObjectTypeQuery1" "ObjectTypeQuery2") true))))