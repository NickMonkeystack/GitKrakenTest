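; Pawn component for the Collaborative Viewer that adds an "Explode" command, triggering the explode animation on a BP_Explode actor.
; BeginPlay caches the first BP_Explode in the level, then post-spawn setup names the command after it and binds a desktop option button.
; The button calls the local pawn's Explode component, relaying through StartAnim_ROS and StartAnim_MTC (server and multicast by naming) to run ExplodeAnim.
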(event Custom|Option1
  ;[1 1 1] Setup Option Buttons
  (bind _asbp_base_pawn (Utilities|Casting|CastToBP_BasePawn (Game|Player|GetPlayerPawn 0)))
  (CallFunction|StartAnimROS (Variables|/Game/CollaborativeViewer/Blueprints/Pawn/BP_BasePawn.BP_BasePawn_C|GetExplode _asbp_base_pawn) (Variables|Default|GetExplodeData)))

(event Custom|StartAnim_ROS
  (params (ExplodeActor :type BP%20Explode%20Object%20Reference))
  (CallFunction|StartAnimMTC ExplodeActor))

(event Custom|StartAnim_MTC
  (params (ExplodeActor :type BP%20Explode%20Object%20Reference))
  (Default|ExplodeAnim ExplodeActor))

(event Custom|Bind_Option_Desktop
  (bind _optionsbuttons (Variables|Default|GetOptionsButtons))
  (bind _output (Utilities|Array|Get(acopy) _optionsbuttons))
  ;[1 1 1] Setup Option Buttons
  (Variables|/Game/CollaborativeViewer/UMG/GameMenu/Option_Button.Option_Button_C|SetWhenExecute _output "NewEnumerator1")
  (EventDispatchers|BindEventtoOnReleased (Variables|/Game/CollaborativeViewer/UMG/GameMenu/Base_Button.Base_Button_C|GetButton _output) (delegate Custom|Option1))
  (EventDispatchers|BindEventtoExecute _output (delegate Custom|Option1)))

(event EventBeginPlay
  (bind _outactors (Actor|GetAllActorsOfClass "/Game/CollaborativeViewer/Blueprints/Commands/Explode/BP_Explode.BP_Explode_C"))
  (Variables|Default|SetExplodeData (Utilities|Array|Get(acopy) _outactors)))

(event EventTick
  (params (DeltaSeconds :type Float%20%28single-precision%29)))

(event EventBeginPlayAfterSpawnPawn
  (Variables|Default|SetOptionsButtonNames (Utilities|Array|MakeArray "Explode"))
  (Variables|Default|SetName (Utilities|Text|ToText(String) (Utilities|GetObjectName (Variables|Default|GetExplodeData))))
  (CallFunction|AddtoDesktopInterface)
  (CallFunction|BindOptionDesktop))