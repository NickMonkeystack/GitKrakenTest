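; Base command component for the Collaborative Viewer that adds a command and its options to the desktop contextual interface.
; AddToDesktopInterface builds an option button widget from each configured name, then creates a named command button that holds those options.
; The command button is added to the ActivateVB of the player controller's contextual widget.
; BeginPlayAfterSpawnPawn is an empty event, and a helper event clears a vertical box's children.
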(event Custom|CreateActivateButton
  ;[1 1 1] Set AcivateButton
  (bind _returnvalue (UserInterface|CreateWidget "/Game/CollaborativeViewer/UMG/GameMenu/Command_Button.Command_Button_C" (Game|GetPlayerController 0)))
  (Variables|/Game/CollaborativeViewer/UMG/GameMenu/Command_Button.Command_Button_C|SetOptions _returnvalue (Variables|Default|GetOptionsButtons))
  (Rendering|Components|TextRender|SetText (Variables|/Game/CollaborativeViewer/UMG/GameMenu/Base_Button.Base_Button_C|GetName _returnvalue) (Variables|Default|GetName))
  (bind _asbp_collab_v_player_controller (Utilities|Casting|CastToBP_Collab_V_PlayerController (Game|GetPlayerController 0)))
  (Variables|Default|SetContextualMenu (Variables|/Game/CollaborativeViewer/Blueprints/PlayerController/BP_Collab_V_PlayerController.BP_Collab_V_PlayerController_C|GetContextualWidget _asbp_collab_v_player_controller))
  (Class|VerticalBox|AddChildtoVerticalBox (Variables|/Game/CollaborativeViewer/UMG/GameMenu/Contextual_Widget.Contextual_Widget_C|GetActivate_VB (Variables|/Game/CollaborativeViewer/Blueprints/PlayerController/BP_Collab_V_PlayerController.BP_Collab_V_PlayerController_C|GetContextualWidget _asbp_collab_v_player_controller)) _returnvalue))

(event Custom|BeginPlayAfterSpawnPawn)

(event Custom|ClearVB
  (params (VB :type Vertical%20Box%20Object%20Reference))
  (for _array_element (Class|PanelWidget|GetAllChildren VB)
    (Widget|RemovefromParent _array_element)))

(event Custom|CreateOptions
  ;[1 1 1] createOption button array
  (CallFunction|CreateOptionButtons (Variables|Default|GetOptionsButtonNames) (Variables|Default|GetOptionsButtons)))

(event Custom|AddToDesktopInterface
  (Utilities|FlowControl|Sequence
    (:then_0
      (Variables|Default|SetOptionNumber (Utilities|Array|Length (Variables|Default|GetOptionsButtonNames))))
    (:then_1
      (CallFunction|CreateOptions)
      (CallFunction|CreateActivateButton))))

(fn CreateOptionButtons
  (params (OptionsNames :type Array%20of%20Texts) (Array :type Array%20of%20Option%20Button%20Object%20References))
  (bind _output_get (LocalVariables|SetOptionsNames_L OptionsNames))
  (for _index (range 0 (- (Utilities|Array|Length _output_get) 1))
    (bind _returnvalue (UserInterface|CreateWidget "/Game/CollaborativeViewer/UMG/GameMenu/Option_Button.Option_Button_C"))
    (Rendering|Components|TextRender|SetText (Variables|/Game/CollaborativeViewer/UMG/GameMenu/Base_Button.Base_Button_C|GetName _returnvalue) (Utilities|Array|Get(acopy) (LocalVariables|GetOptionsNames_L) _index))
    (Utilities|Array|Add Array _returnvalue)))